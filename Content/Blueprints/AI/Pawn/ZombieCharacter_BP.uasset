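; Zombie AI character with an overhead-style health bar widget and a switchable movement speed.
; Every Tick it pushes the HealthComponent's health ratio into the UMG_HealthBar, showing the widget only while the first player's pawn is within range.
; A ChangeZombieMoveSpeed event takes a boolean to toggle the max walk speed between a slow walk and a fast run.
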(event `self.ReceiveTick`
  (params (DeltaSeconds :type "Float (single-precision)"))
  (bind _healthcomponent (`self.HealthComponent`))
  (bind _asumg_health_bar (cast `/Game/Blueprints/UMG/UMG_HealthBar` (`WidgetComponent.GetWidget` (`self.HealthBarWidget`))))
  (`ProgressBar.SetPercent` (`/Game/Blueprints/UMG/UMG_HealthBar.HealhBar` _asumg_health_bar) (/ (`HealthComponent.CurrentHealth` _healthcomponent) (`HealthComponent.MaxHealth` _healthcomponent)))
  (if (<= (`KismetMathLibrary.Vector_Distance` (`self.K2_GetActorLocation`) (`self.K2_GetActorLocation` (`GameplayStatics.GetPlayerPawn` 0))) 1000.0)
    (set `Widget.Visibility` "Visible" _asumg_health_bar)
    (else
      (set `Widget.Visibility` "Hidden" _asumg_health_bar))))

(event `self.ChangeZombieMoveSpeed`
  (params (Decision :type Boolean))
  (if Decision
    (set `CharacterMovementComponent.MaxWalkSpeed` 500.0 (`self.CharacterMovement`))
    (else
      (set `CharacterMovementComponent.MaxWalkSpeed` 100.0 (`self.CharacterMovement`)))))

(fn `UserConstructionScript`)