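; Behavior tree task that moves an AI pawn to a random location while watching for a detected player.
; On execute, AI MoveTo heads for the RandomMoveToLocation blackboard vector and finishes the task with the move's success or failure.
; Each tick, it fails the task early if the TargetActor blackboard value casts to MyCharacter_BP, without explicitly stopping the move.
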(event `self.ReceiveTickAI`
  (params (OwnerController :type "AIController Object Reference") (ControlledPawn :type "Pawn Object Reference") (DeltaSeconds :type "Float (single-precision)"))
  (cast `/Game/Blueprints/Pawn/MyCharacter_BP` (`BlackboardComponent.GetValueAsObject` (`AIBlueprintHelperLibrary.GetBlackboard` ControlledPawn) "TargetActor"))
  (`self.FinishExecute` false))

(event `self.ReceiveExecuteAI`
  (params (OwnerController :type "AIController Object Reference") (ControlledPawn :type "Pawn Object Reference"))
  (`|AIMoveTo` ControlledPawn (`BlackboardComponent.GetValueAsVector` (`AIBlueprintHelperLibrary.GetBlackboard` ControlledPawn) "RandomMoveToLocation") null
    (:`OnSuccess`
      (`self.FinishExecute` true))
    (:`OnFail`
      (`self.FinishExecute` false))))